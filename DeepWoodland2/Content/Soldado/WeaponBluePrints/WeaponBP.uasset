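; Pickup weapon actor that the player character can equip, holster, drop and switch between long and short types.
; Overlapping its collision enables input and highlights it with a widget and custom depth.
; Equip holsters the current weapon, drops any sharing its secondary socket, then snaps this one to the primary socket and updates the ThirdPersonCharacter's armed state.
; Select picks long or short by fixed attached-actor index, with FlipFlop cycling.
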(event `self.Colission.OnComponentBeginOverlap`
  (params (OverlappedComponent :type "PrimitiveComponent Object Reference") (OtherActor :type "Actor Object Reference") (OtherComp :type "PrimitiveComponent Object Reference") (OtherBodyIndex :type Integer) (bFromSweep :type Boolean) (SweepResult :type "HitResult Structure (by ref)"))
  ;[1 1 1] Activa el uso de teclado cuando se acerca a un arma
  (`self.InputEnable` true)
  (`self.Highlight` true))

(event `self.Colission.OnComponentEndOverlap`
  (params (OverlappedComponent :type "PrimitiveComponent Object Reference") (OtherActor :type "Actor Object Reference") (OtherComp :type "PrimitiveComponent Object Reference") (OtherBodyIndex :type Integer))
  ;[1 1 1] Desactiva el uso de teclado cuando no tiene armas
  (bind _asthird_person_character (cast `/Game/ThirdPersonBP/Blueprints/ThirdPersonCharacter` (`GameplayStatics.GetPlayerCharacter` 0)))
  (if (not (`/Game/ThirdPersonBP/Blueprints/ThirdPersonCharacter.IsArmed_BP` _asthird_person_character))
    (`self.InputEnable` false))
  (`self.Highlight` false))

(event `InputAction|Drop`
  (params (Key :type "Key Structure"))
  ;[1 1 1] Funcion para soltar arma
  (:`Pressed`
    (`self.Drop` null)))

(event `InputAction|Equip`
  (params (Key :type "Key Structure"))
  ;[1 1 1] Funcion para equipar arma
  (:`Pressed`
    (`self.Equip`)))

(event `InputAction|Keep`
  (params (Key :type "Key Structure"))
  ;[1 1 1] Funcion para colocar arma en el cuerpo
  (:`Pressed`
    (`self.Keep`)))

(event `InputAction|LongWeapon`
  (params (Key :type "Key Structure"))
  ;[1 1 1] Arma Larga
  (:`Pressed`
    (`self.Select` "LONG" :!label _label)))

(event `InputAction|ShortWeapon`
  (params (Key :type "Key Structure"))
  ;[1 1 1] Arma Corta
  (:`Pressed`
    (`self.Select` "SHORT" :!label _label_2)))

(event `InputAction|NextWeapon`
  (params (Key :type "Key Structure"))
  ;[1 1 1] Permite intercambiar entre armas cortas y largas
  (:`Pressed`
    (`/Engine/EditorBlueprintResources/StandardMacros.FlipFlop`
      (:`A`
        (goto _label))
      (:`B`
        (goto _label_2)))))

(fn `Drop`
  (params (Weapon :type "/Game/Soldado/WeaponBluePrints/WeaponBP Object Reference"))
  ;[1 1 1] Ingresa
  (bind _asthird_person_character (cast `/Game/ThirdPersonBP/Blueprints/ThirdPersonCharacter` (`GameplayStatics.GetPlayerCharacter` 0)))
  ;[1 1 1] Indica que NO tiene arma
  (set `/Game/ThirdPersonBP/Blueprints/ThirdPersonCharacter.IsArmed_BP` false _asthird_person_character)
  (set `/Game/ThirdPersonBP/Blueprints/ThirdPersonCharacter.CurrentWeapon` null _asthird_person_character)
  (`/Engine/EditorBlueprintResources/StandardMacros.IsValid` Weapon
    (:`Is Valid`
      ;[1 1 1] Parametro valido = liberar arma indicada
      (`self.K2_DetachFromActor` Weapon "KeepWorld" "KeepWorld" "KeepWorld"))
    (:`Is Not Valid`
      ;[1 1 1] Parametro NO valido = liberar arma actual
      (`self.K2_DetachFromActor` "KeepWorld" "KeepWorld" "KeepWorld")))
  (`PrimitiveComponent.SetCollisionEnabled` (`self.Colission`) "QueryOnly"))

(fn `Equip`
  (locals (TPC :type "/Game/ThirdPersonBP/Blueprints/ThirdPersonCharacter Object Reference"))
  (bind _tpc (`local.TPC`))
  ;[1 1 1] Guarda el arma en mano
  (`self.Keep`)
  (bind _asthird_person_character (cast `/Game/ThirdPersonBP/Blueprints/ThirdPersonCharacter` (`GameplayStatics.GetPlayerCharacter` 0)))
  (bind _output_get (set `local.TPC` _asthird_person_character))
  (for _array_element (`self.GetAttachedActors` _output_get true)
    (bind _asweapon_bp (cast `/Game/Soldado/WeaponBluePrints/WeaponBP` _array_element))
    ;[1 1 1] 2 armas, mismo socket, se libera una
    (if (== (`/Game/Soldado/WeaponBluePrints/WeaponBP.SecondarySocket` _asweapon_bp) (`self.SecondarySocket`))
      (`self.Drop` _asweapon_bp null)))
  (`self.K2_AttachToComponent` self (`Character.Mesh` (`local.TPC`)) (`self.PrimarySocket`) "SnapToTarget" "SnapToTarget" "SnapToTarget" true)
  ;[0.9926 1 0.4199] Indica que está armado
  (set `/Game/ThirdPersonBP/Blueprints/ThirdPersonCharacter.IsArmed_BP` true _tpc)
  (set `/Game/ThirdPersonBP/Blueprints/ThirdPersonCharacter.CurrentWeapon` self _tpc)
  (`PrimitiveComponent.SetCollisionEnabled` (`self.Colission`) "NoCollision"))

(fn `Highlight`
  (params (Show :type Boolean) (Weapon :type "/Game/Soldado/WeaponBluePrints/WeaponBP Object Reference"))
  (locals (V_weapon :type "/Game/Soldado/WeaponBluePrints/WeaponBP Object Reference"))
  (bind _v_weapon (`local.V_weapon`))
  (bind _output_get (set `local.V_weapon` Weapon))
  (if (not (`KismetSystemLibrary.IsValid` _output_get))
    (set `local.V_weapon` self))
  (`SceneComponent.SetVisibility` (`/Game/Soldado/WeaponBluePrints/WeaponBP.Widget` _v_weapon) Show false)
  (`PrimitiveComponent.SetRenderCustomDepth` (`/Game/Soldado/WeaponBluePrints/WeaponBP.Weapon` _v_weapon) Show))

(fn `InputEnable`
  (params (Enable :type Boolean))
  (bind _returnvalue (`GameplayStatics.GetPlayerController` 0))
  ;[1 0.7969 0] Activa/Desactiva el uso de las teclas para el arma
  (if Enable
    (`self.EnableInput` _returnvalue)
    (else
      (`self.DisableInput` _returnvalue))))

(fn `Keep`
  (bind _returnvalue (`GameplayStatics.GetPlayerCharacter` 0))
  ;[1 1 1] Referencia al personaje
  (bind _asthird_person_character (cast `/Game/ThirdPersonBP/Blueprints/ThirdPersonCharacter` _returnvalue))
  (bind _currentweapon (`/Game/ThirdPersonBP/Blueprints/ThirdPersonCharacter.CurrentWeapon` _asthird_person_character))
  (`/Engine/EditorBlueprintResources/StandardMacros.IsValid` _currentweapon
    (:`Is Valid`
      ;[1 1 1] Socket en donde está
      (`self.K2_AttachToComponent` _currentweapon (`Character.Mesh` _returnvalue) (`/Game/Soldado/WeaponBluePrints/WeaponBP.SecondarySocket` _currentweapon) "SnapToTarget" "SnapToTarget" "SnapToTarget" true)
      ;[1 1 1] indica que no tiene armas
      (set `/Game/ThirdPersonBP/Blueprints/ThirdPersonCharacter.IsArmed_BP` false _asthird_person_character)
      (set `/Game/ThirdPersonBP/Blueprints/ThirdPersonCharacter.CurrentWeapon` self _asthird_person_character))))

(fn `Select`
  (params (WeaponType :type String))
  (locals (TPC :type "/Game/ThirdPersonBP/Blueprints/ThirdPersonCharacter Object Reference") (TPCMesh :type "SkeletalMeshComponent Object Reference"))
  (bind _returnvalue (`GameplayStatics.GetPlayerCharacter` 0))
  (bind _tpcmesh (`local.TPCMesh`))
  (bind _primarysocket (`self.PrimarySocket`))
  (bind _tpc (`local.TPC`))
  ;[1 1 1] Se guarda el arma
  (`self.Keep`)
  (bind _asthird_person_character (cast `/Game/ThirdPersonBP/Blueprints/ThirdPersonCharacter` _returnvalue))
  (set `local.TPC` _asthird_person_character)
  (set `local.TPCMesh` (`Character.Mesh` _returnvalue))
  (if (`KismetStringLibrary.EqualEqual_StrStr` WeaponType "LONG")
    ;[1 1 1] Arma Larga = primera posicion
    (bind _asweapon_bp (cast `/Game/Soldado/WeaponBluePrints/WeaponBP` (`|GetArrayItem` (`self.GetAttachedActors` (`local.TPC`) true) 1)))
    (`self.K2_AttachToComponent` _asweapon_bp _tpcmesh _primarysocket "SnapToTarget" "SnapToTarget" "SnapToTarget" true)
    (set `/Game/ThirdPersonBP/Blueprints/ThirdPersonCharacter.CurrentWeapon` _asweapon_bp _tpc)
    (else
      ;[1 1 1] Arma corta
      (bind _asweapon_bp_2 (cast `/Game/Soldado/WeaponBluePrints/WeaponBP` (`|GetArrayItem` (`self.GetAttachedActors` (`local.TPC`) true))))
      (`self.K2_AttachToComponent` _asweapon_bp_2 _tpcmesh _primarysocket "SnapToTarget" "SnapToTarget" "SnapToTarget" true)
      (set `/Game/ThirdPersonBP/Blueprints/ThirdPersonCharacter.CurrentWeapon` _asweapon_bp_2 _tpc)))
  (set `/Game/ThirdPersonBP/Blueprints/ThirdPersonCharacter.IsArmed_BP` true _tpc))

(fn `UserConstructionScript`)