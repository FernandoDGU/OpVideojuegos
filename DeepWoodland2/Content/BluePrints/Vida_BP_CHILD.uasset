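; Child item Blueprint that acts as a health pickup, raising the player's Vida (health) when the object is used.
; Its UsarObjeto override runs the parent logic, casts player 0's character to ThirdPersonCharacter, adds a fixed amount to Vida with no clamp, and returns true.
; All other behavior comes from the parent class, as its event nodes are disabled stubs and its construction script only calls the parent.
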(fn `UsarObjeto`
  (returns (Use :type Boolean))
  (`parent.UsarObjeto`)
  (bind _asthird_person_character (cast `/Game/ThirdPersonBP/Blueprints/ThirdPersonCharacter` (`GameplayStatics.GetPlayerCharacter` 0)))
  (set `/Game/ThirdPersonBP/Blueprints/ThirdPersonCharacter.Vida` (+ (`/Game/ThirdPersonBP/Blueprints/ThirdPersonCharacter.Vida` _asthird_person_character) 25.0) _asthird_person_character)
  (return true))

(fn `UserConstructionScript`
  (`parent.UserConstructionScript`))