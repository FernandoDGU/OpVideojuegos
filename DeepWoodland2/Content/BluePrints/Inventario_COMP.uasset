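; Inventory component that stores items in a fixed-size slot array and toggles a centered inventory window on the player controller's HUD canvas.
; AñadirAInventario merges stackable items into a non-full stack of the same class found by ApilarMacro, otherwise CrearPila writes to the first empty slot.
; AddPila caps stacks at the item's maximum and recursively re-adds any overflow.
; AñadirAInventario always returns false.
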(event `self.ReceiveBeginPlay`
  (`self.IniciarInventario`))

(fn `AbrirCerrar`
  (bind _ventanainventario (`self.VentanaInventario`)
    (:`then`
      (`Widget.RemoveFromParent` _ventanainventario)
      (set `self.VentanaInventario` null)
      (set `PlayerController.bShowMouseCursor` false (`GameplayStatics.GetPlayerController` 0)))
    (:`else`
      (bind _returnvalue (`|CreateWidget` "/Game/Widgets/Inventario_Ventana.Inventario_Ventana_C" (`GameplayStatics.GetPlayerController` 0) self))
      (set `self.VentanaInventario` _returnvalue)
      (bind _ascontrolador_jugador (cast `/Game/BluePrints/Controlador_Jugador` (`GameplayStatics.GetPlayerController` 0)))
      (bind _returnvalue_2 (`CanvasPanel.AddChildToCanvas` (`/Game/Widgets/HUD.HUDLienzo` (`/Game/BluePrints/Controlador_Jugador.HUDPantalla` _ascontrolador_jugador)) (`self.VentanaInventario`)))
      (`CanvasPanelSlot.SetAutoSize` _returnvalue_2 true)
      (`CanvasPanelSlot.SetAlignment` _returnvalue_2 (0.5 0.5))
      (`CanvasPanelSlot.SetAnchors` _returnvalue_2 (make `Anchors` (0.5 0.5) (0.5 0.5)))
      (`CanvasPanelSlot.SetPosition` _returnvalue_2 (`self.Posicion`)))))

(fn `AddPila`
  (params (EstructuraEspacio :type "/Game/BluePrints/Espacio_STR Structure") (EspacioIndice :type Integer))
  (bind _espacioindice (`local.EspacioIndice`))
  (bind (_estructuraespacio_objetoestructura _estructuraespacio_cantidad) (break `/Game/BluePrints/Espacio_STR` (`local.EstructuraEspacio`)))
  (bind _inventario (`self.Inventario`))
  (bind _estructuraespacio_objetoestructura_2 (break `/Game/BluePrints/Espacio_STR` (`local.EstructuraEspacio`)))
  (bind (_estructuraespacio_objetoestructura_3 _estructuraespacio_cantidad_2) (break `/Game/BluePrints/Espacio_STR` (`local.EstructuraEspacio`)))
  (bind (_nombre _apilable _imagen _max_apilar) (break `/Game/BluePrints/Objeto_STR` _estructuraespacio_objetoestructura_2))
  (bind _output (`|GetArrayItem` (`self.Inventario`) EspacioIndice))
  (bind (_output_objetoestructura _output_cantidad) (break `/Game/BluePrints/Espacio_STR` (`|GetArrayItem` _inventario _espacioindice)))
  (bind _output_get (set `self.CantidadActual` (`.Cantidad_6_D4A6251647E383CAA86DC2ACD061DFED` (break `/Game/BluePrints/Espacio_STR` _output))))
  (if (> (+ (`.Cantidad_6_D4A6251647E383CAA86DC2ACD061DFED` (break `/Game/BluePrints/Espacio_STR` EstructuraEspacio)) _output_get) (`.Max_Apilar_11_F5F5978F4BA6C8B8EB0197BD313DEEC7` (break `/Game/BluePrints/Objeto_STR` (break `/Game/BluePrints/Espacio_STR` _output))))
    (`KismetArrayLibrary.Array_Set` (`self.Inventario`) (`local.EspacioIndice`) (make `/Game/BluePrints/Espacio_STR` _estructuraespacio_objetoestructura_2 _max_apilar))
    (`self.AñadirAInventario` (make `/Game/BluePrints/Espacio_STR` _estructuraespacio_objetoestructura_3 (- _estructuraespacio_cantidad_2 (- _max_apilar (`self.CantidadActual`)))))
    (else
      (`KismetArrayLibrary.Array_Set` _inventario _espacioindice (make `/Game/BluePrints/Espacio_STR` _output_objetoestructura (+ _estructuraespacio_cantidad _output_cantidad)))))
  (return))

(fn `AñadirAInventario`
  (params (ContenidoAdd :type "/Game/BluePrints/Espacio_STR Structure"))
  (returns (AddQuestion :type Boolean))
  (bind _contenidoadd (`local.ContenidoAdd`))
  (if (`.Apilable_6_5A3ABD354925E8FB26596784B4FE8B36` (break `/Game/BluePrints/Objeto_STR` (break `/Game/BluePrints/Espacio_STR` ContenidoAdd)))
    (bind _indiceapilar (`self.ApilarMacro` _contenidoadd)
      (:`Verdadero`
        (`self.AddPila` (`local.ContenidoAdd`) _indiceapilar))
      (:`Falso`
        (`self.CrearPila` _contenidoadd :!label _label)))
    (else
      (goto _label)))
  (return false))

(fn `CrearPila`
  (params (ContenidoADD :type "/Game/BluePrints/Espacio_STR Structure"))
  (`KismetArrayLibrary.Array_Set` (`self.Inventario`) (`KismetArrayLibrary.Array_Find` (`self.Inventario`) (make `/Game/BluePrints/Espacio_STR` (struct :`Nombre` "NULL" :`Apilable` true :`Max_Apilar` 5))) ContenidoADD))

(fn `IniciarInventario`
  (`KismetArrayLibrary.Array_Resize` (`self.Inventario`) (`self.Espacio`)))