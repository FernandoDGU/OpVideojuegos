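; BP_Gate is a double gate that swings open when something enters its Box trigger and closes again when it leaves.
; Overlap begin plays the Right and Left timelines, each setting the yaw of its door mesh, and overlap end reverses both.
; Rotation is set in world space with zero pitch and roll, and the overlaps do not filter which actor triggers them.
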(event `self.Box.OnComponentBeginOverlap`
  (params (OverlappedComponent :type "PrimitiveComponent Object Reference") (OtherActor :type "Actor Object Reference") (OtherComp :type "PrimitiveComponent Object Reference") (OtherBodyIndex :type Integer) (bFromSweep :type Boolean) (SweepResult :type "HitResult Structure (by ref)"))
  (`|ExecutionSequence`
    (:`then_0`
      (bind (_direction _newtrack_0) (`Timeline|right` :`NewTime` 5.0 :!label _label)
        (:`Update`
          (`SceneComponent.K2_SetWorldRotation` (`self.RightDoor`) (`KismetMathLibrary.MakeRotator` 0.0 0.0 _newtrack_0) false false))))
    (:`then_1`
      (bind (_direction_2 _newtrack_0_2) (`Timeline|left` :!label _label_2)
        (:`Update`
          (`SceneComponent.K2_SetWorldRotation` (`self.LeftDoor`) (`KismetMathLibrary.MakeRotator` 0.0 0.0 _newtrack_0_2) false false))))))

(event `self.Box.OnComponentEndOverlap`
  (params (OverlappedComponent :type "PrimitiveComponent Object Reference") (OtherActor :type "Actor Object Reference") (OtherComp :type "PrimitiveComponent Object Reference") (OtherBodyIndex :type Integer))
  (`|ExecutionSequence`
    (:`then_0`
      (goto _label :!via `Reverse`))
    (:`then_1`
      (goto _label_2 :!via `Reverse`))))

(fn `UserConstructionScript`)